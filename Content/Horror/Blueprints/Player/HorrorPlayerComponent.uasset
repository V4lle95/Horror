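; Player component for the horror game that provides camera zoom for the owning Character.
; On BeginPlay it caches the owner, its movement component and, if a camera reference is valid, that camera's default field of view.
; ZoomIn steps a clamped zoom factor and converts it to a field of view through the half-angle tangent, treating the factor as true magnification.
; ZoomOut is an empty stub.
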(event Custom|Zoom%20In
  (CallFunction|ModifyZoomFactor (Variables|Default|GetZoom%20Step))
  (bind _fov (CallFunction|CalculateFoVforZoomValue (Variables|Default|GetZoomFactor)))
  (Camera|SetFieldOfView (Variables|Default|GetOwner%20Camera) _fov))

(event Custom|Zoom%20Out)

(event EventBeginPlay
  (bind _owner_camera (Variables|Default|GetOwner%20Camera))
  (bind _ascharacter (Utilities|Casting|CastToCharacter (Components|GetOwner)))
  (bind _output_get (Variables|Default|SetOwner _ascharacter))
  (Variables|Default|SetOwner%20Movement (Variables|/Script/Engine.Character|GetCharacterMovement _output_get))
  (Utilities|IsValid _owner_camera
    (:Is%20Valid
      (Variables|Default|SetDefaultFieldOfView (Variables|/Script/Engine.CameraComponent|GetFieldOfView _owner_camera)))))

(fn ModifyZoomFactor
  (params (Delta :type Float%20%28single-precision%29))
  (Variables|Default|SetZoomFactor (Math|Float|Clamp(Float) (+ (Variables|Default|GetZoomFactor) Delta) (Variables|Default|GetMinZoom) (Variables|Default|GetMaxZoom)))
  (return))

(fn CalculateFoVforZoomValue
  (params (Zoom%20Facter :type Float%20%28single-precision%29))
  (return (* (Class|KismetMathLibrary|DegAtan (/ (Math|Trig|Tan(Degrees) (/ (Variables|Default|GetDefaultFieldOfView) 2.0)) Zoom%20Facter)) 2.0)))