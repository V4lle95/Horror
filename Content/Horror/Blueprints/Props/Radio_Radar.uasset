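; Radio radar prop for the horror game that shows the nearest BP_AI on its screen material.
; A fast looping timer finds the AI nearest the player, or switches the screen to a noise material when none is found.
; Player-to-AI distance and the look-at yaw from the radar, combined with its own rotation, drive the material's scalar parameters.
; Each successful check recreates the screen's dynamic material instance.
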(event Custom|Check%20For%20AI
  (bind (_success _nearestactorofclass) (CallFunction|NearestActortoPlayerOfClass "/Game/Horror/Blueprints/AI/BP_AI.BP_AI_C"))
  (if _success
    (if (!= (* (/ (Transformation|GetDistanceTo (Game|Player|GetPlayerPawn 0) _nearestactorofclass) 52.5) 0.01) 0.0)
      (Rendering|Material|SetMaterial (Variables|Default|GetRadar) 1 "/Game/Horror/Materials/Search_Radar_M_Inst.Search_Radar_M_Inst")
      (bind _returnvalue (Rendering|Material|CreateDynamicMaterialInstance (Variables|Default|GetRadar) 1 "/Game/Horror/Materials/Search_Radar_M_Inst.Search_Radar_M_Inst" "None" :!class /Script/Engine.PrimitiveComponent))
      (Variables|Default|SetRadar%20Material _returnvalue)
      (Rendering|Material|SetScalarParameterValue (Variables|Default|GetRadar%20Material) "Disntace" (Math|Float|Lerp 1.0 0.0 (* (/ (Transformation|GetDistanceTo (Game|Player|GetPlayerPawn 0) _nearestactorofclass) 52.5) 0.01)) :!class /Script/Engine.MaterialInstanceDynamic)
      (Rendering|Material|SetScalarParameterValue (Variables|Default|GetRadar%20Material) "Rotation" (* (.yaw (Math|Rotator|CombineRotators (Math|Rotator|FindLookatRotation (Transformation|GetActorLocation) (Transformation|GetActorLocation _nearestactorofclass)) (Transformation|GetActorRotation))) -1.0) :!class /Script/Engine.MaterialInstanceDynamic)
      (else
        (Rendering|Material|SetMaterial (Variables|Default|GetRadar) 1 "/Game/Horror/Materials/Search_Radar_M_Inst.Search_Radar_M_Inst")
        (bind _returnvalue_2 (Rendering|Material|CreateDynamicMaterialInstance (Variables|Default|GetRadar) 1 "/Game/Horror/Materials/Search_Radar_M_Inst.Search_Radar_M_Inst" "None" :!class /Script/Engine.PrimitiveComponent))
        (bind _output_get (Variables|Default|SetRadar%20Material _returnvalue_2))
        (Rendering|Material|SetScalarParameterValue _returnvalue_2 "Disntace" 0.0 :!class /Script/Engine.MaterialInstanceDynamic)
        (Rendering|Material|SetScalarParameterValue (Variables|Default|GetRadar%20Material) "Rotation" 0.0 :!class /Script/Engine.MaterialInstanceDynamic)))
    (else
      (Rendering|Material|SetMaterial (Variables|Default|GetRadar) 1 "/Game/Horror/Materials/Noise_M_Inst.Noise_M_Inst"))))

(event EventBeginPlay
  (Utilities|Time|SetTimerbyFunctionName 0 "Check For AI" 0.01 true))

(event Collision|EventActorBeginOverlap
  (params (OtherActor :type Actor%20Object%20Reference)))

(fn ConstructionScript
  (|CallParentFunction)
  (bind _returnvalue (Rendering|Material|CreateDynamicMaterialInstance (Variables|Default|GetRadar) 1 "/Game/Horror/Materials/Search_Radar_M_Inst.Search_Radar_M_Inst" "None" :!class /Script/Engine.PrimitiveComponent))
  (Variables|Default|SetRadar%20Material _returnvalue))