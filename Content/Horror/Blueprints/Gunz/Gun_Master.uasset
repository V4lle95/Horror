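; Base gun actor that aims at the mouse cursor and fires hitscan shots.
; A fast looping timer started on BeginPlay rotates the gun toward a distant point along the deprojected cursor ray.
; The Fire event line-traces from the Scene component along that aim against pawns and world objects, applying damage to the hit actor.
; The trace still has timed debug drawing enabled.
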(event Custom|Pistol%20Rotation
  (bind _returnvalue (Game|GetPlayerController 0))
  (bind (_worldlocation _worlddirection) (Game|Player|ConvertMouseLocationToWorldSpace _returnvalue))
  (Transformation|SetActorRotation (Math|Rotator|FindLookatRotation (Transformation|GetActorLocation) (+ _worldlocation (* _worlddirection 5e+03)))))

(event EventBeginPlay
  (Utilities|Time|SetTimerbyEvent (delegate Custom|Pistol%20Rotation) 0.01 true))

(event EventFire
  (bind _returnvalue (Game|GetPlayerController 0))
  (bind (_worldlocation _worlddirection) (Game|Player|ConvertMouseLocationToWorldSpace _returnvalue))
  (bind (_outhit _returnvalue_2) (Collision|LineTraceForObjects (Transformation|GetWorldLocation (Variables|Default|GetScene)) (+ _worldlocation (* _worlddirection 1.5e+03)) (Utilities|Array|MakeArray "ObjectTypeQuery3" "ObjectTypeQuery1" "ObjectTypeQuery2") true (Utilities|Array|MakeArray self 0) "ForDuration"))
  (if _returnvalue_2
    (Game|Damage|ApplyDamage (.hitactor _outhit) 1.0 0 self)))

(fn ConstructionScript
  (|CallParentFunction))