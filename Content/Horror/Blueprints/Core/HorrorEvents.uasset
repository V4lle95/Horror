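; HorrorEvents is the horror game's core player controller logic, driving movement, look, camera and interaction on the player's pawn from outside it.
; BeginPlay creates the HUD, re-parents the tagged camera onto a runtime spring arm and starts looping function timers.
; Timers drive walking head shake, distance-based footsteps by physical surface and a usable-object check.
; Use inputs sphere-trace from the camera to message hit actors; Reset Camera eases the view forward.
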(event EventBeginPlay
  (Utilities|FlowControl|Sequence
    (:then_0
      (bind _returnvalue (UserInterface|CreateWidget "/Game/Horror/Blueprints/Widgets/HUD_w.HUD_w_C"))
      (bind _output_get (Variables|Default|SetHUD%20w _returnvalue))
      (UserInterface|Viewport|AddtoViewport _output_get 0)
      (Input|EnableInput (Game|GetPlayerController 0))
      (Utilities|Time|SetTimerbyFunctionName 0 "Footsteps/HeadShake" 0.1 true)
      (Utilities|Time|SetTimerbyFunctionName 0 "Turn viewport" 0.01 true)
      (bind _output_get_2 (Variables|Default|SetPlayerCamera (Utilities|Array|Get(acopy) (Actor|GetComponentsbyTag (Game|Player|GetPlayerPawn 0) "/Script/Engine.CameraComponent" "Camera"))))
      (Utilities|IsValid _output_get_2
        (:Is%20Valid
          (Camera|SetFieldOfView _output_get_2 (Variables|DOF|GetDefaultFOV))
          (bind _returnvalue_2 (AddComponent|AddSpringArmComponent (Game|Player|GetPlayerPawn 0) false (Transformation|GetRelativeTransform (Variables|Default|GetPlayerCamera))))
          (bind _output_get_3 (Variables|Default|SetCameraSpringArm _returnvalue_2))
          (bind _asspring_arm_component (Utilities|Casting|CastToSpringArmComponent _output_get_3))
          (Variables|Movement|SetCameraSpringArmHeight (.z (Variables|/Script/Engine.SceneComponent|GetRelativeLocation _asspring_arm_component)))
          (bind _output_get_4 (Variables|/Script/Engine.SpringArmComponent|SetbUsePawnControlRotation _asspring_arm_component true))
          (Variables|/Script/Engine.SpringArmComponent|SetbEnableCameraRotationLag _asspring_arm_component _output_get_4)
          (Variables|/Script/Engine.SpringArmComponent|SetTargetArmLength _asspring_arm_component 0.0)
          (Variables|/Script/Engine.SpringArmComponent|SetCameraRotationLagSpeed _asspring_arm_component 0.0)
          (Variables|/Script/Engine.SpringArmComponent|SetProbeChannel _asspring_arm_component "ECC_WorldStatic")
          (Variables|/Script/Engine.SpringArmComponent|SetProbeSize _asspring_arm_component 0.0)
          (Variables|/Script/Engine.CameraComponent|SetbUsePawnControlRotation (Variables|Default|GetPlayerCamera) false)
          (Transformation|AttachComponentToComponent (Variables|Default|GetPlayerCamera) (Variables|Default|GetCameraSpringArm) "None" "SnapToTarget" "SnapToTarget" "SnapToTarget" true))))
    (:then_1
      (Utilities|Time|SetTimerbyFunctionName 0 "CheckUse" 0.01 true))))

(event Input|ActionEvents|InputActionUse
  (params (Key :type Key%20Structure))
  ;[1 1 1] InputAction Settings
  (:Pressed
    (bind _hit_actor (Utilities|GetUsable)
      (:execute
        (Class|HorrorInterfaceBPI|Use(Message) _hit_actor)))))

(event Input|ActionEvents|InputActionAlternativeUse
  (params (Key :type Key%20Structure))
  ;[1 1 1] InputAction Settings
  (:Pressed
    (bind _hit_actor (Utilities|GetUsable)
      (:execute
        (Class|HorrorInterfaceBPI|AlternativeUse(Message) _hit_actor)))))

(event Input|ActionEvents|InputActionResetCamera
  (params (Key :type Key%20Structure))
  ;[1 1 1] InputAction Settings
  (:Pressed
    (CallFunction|ResetCameraPosition)))

(event Custom|Reset%20Camera%20Position
  (bind _returnvalue (Game|GetPlayerCharacter 0))
  (Variables|Default|SetCamera%20Current%20ROT (Pawn|GetControlRotation _returnvalue :!class /Script/Engine.Pawn))
  (bind _alpha (Timeline|Camera%20Rot PlayFromStart)
    (:Update
      (Pawn|SetControlRotation (Game|GetPlayerController 0) (Math|Rotator|Lerp(Rotator) (Variables|Default|GetCamera%20Current%20ROT) (Math|Conversions|RotationFromXVector (Transformation|GetActorForwardVector _returnvalue)) _alpha true)))))

(event Input|AxisEvents|InputAxisMoveRight
  (params (AxisValue :type Float%20%28single-precision%29))
  (if (!= AxisValue 0.0)
    (Pawn|Input|AddMovementInput (Game|GetPlayerCharacter 0) (Transformation|GetActorRightVector (Game|GetPlayerCharacter 0)) AxisValue false)))

(event Input|AxisEvents|InputAxisMoveForward
  (params (AxisValue :type Float%20%28single-precision%29))
  (if (!= AxisValue 0.0)
    (Pawn|Input|AddMovementInput (Game|GetPlayerCharacter 0) (Transformation|GetActorForwardVector (Game|GetPlayerCharacter 0)) AxisValue false)))

(event Input|AxisEvents|InputAxisLookUp
  (params (AxisValue :type Float%20%28single-precision%29))
  (Pawn|Input|AddControllerPitchInput (Game|GetPlayerCharacter 0) AxisValue))

(event Input|AxisEvents|InputAxisTurn
  (params (AxisValue :type Float%20%28single-precision%29))
  (Pawn|Input|AddControllerYawInput (Game|GetPlayerCharacter 0) AxisValue))

(fn ConstructionScript)

(fn Footsteps/HeadShake
  (bind _returnvalue (Game|Player|GetPlayerPawn 0))
  (bind _returnvalue_2 (Game|Player|GetPlayerPawn 0))
  (bind _returnvalue_3 (Transformation|GetActorLocation _returnvalue_2))
  (if (and (AI|Components|NavMovement|IsMovingonGround (Pawn|GetMovementComponent _returnvalue)) (>= (Math|Vector|VectorLength (Transformation|GetVelocity _returnvalue)) 5e+01))
    (Class|PlayerController|ClientPlayCameraShake (Game|GetPlayerController 0) "/Game/Horror/Blueprints/Player/HeadShakeWalking.HeadShakeWalking_C" 1.0 "CameraLocal" "0, 0, 0")
    (if (and (> (Math|Vector|VectorLength (- (Transformation|GetActorLocation _returnvalue_2) (Variables|Default|GetCurrentFootLocation))) (Variables|Default|GetStep%20Size)) (AI|Components|NavMovement|IsMovingonGround (Pawn|GetMovementComponent _returnvalue_2)))
      (bind (_outhit _returnvalue_4) (Collision|SphereTraceByChannel _returnvalue_3 (- _returnvalue_3 (* (Transformation|GetActorUpVector _returnvalue_2) 1.5e+02)) 3e+01 "TraceTypeQuery1" false 0 "None"))
      (if _returnvalue_4
        (Variables|Default|SetCurrentFootLocation (.Location (Collision|BreakHitResult _outhit)))
        (Audio|SpawnSound2D (Utilities|Select :Index (Variables|/Script/Engine.PhysicalMaterial|GetSurfaceType (.PhysMat (Collision|BreakHitResult _outhit))) :SurfaceType_Default "/Game/Horror/Sounds/Female_Voice/heel-reverb2.heel-reverb2" :SurfaceType1 0 :SurfaceType2 "/Game/Horror/Sounds/stepdirt_4.stepdirt_4" :SurfaceType3 "/Game/Horror/Sounds/grassy-footstep4.grassy-footstep4" :SurfaceType4 "/Game/Horror/Sounds/Female_Voice/heel-reverb4.heel-reverb4" :SurfaceType5 "/Game/Horror/Sounds/272307__sturmankin__concrete-09d-highheels-onoff.272307__sturmankin__concrete-09d-highheels-onoff" :SurfaceType6 "/Game/Horror/Sounds/Female_Voice/heel-reverb4.heel-reverb4" :SurfaceType7 "/Game/Horror/Sounds/stepwood_2.stepwood_2") 1.0 1.0 0.0 0)))))

(fn CheckUse
  (bind _playercamera (Variables|Default|GetPlayerCamera))
  (bind _returnvalue (Transformation|GetWorldLocation _playercamera))
  (bind _outactors (Actor|GetAllActorswithTag "IgnoreTrace"))
  (bind (_outhit _returnvalue_2) (Collision|SphereTraceByChannel _returnvalue (+ _returnvalue (* (Math|Vector|GetForwardVector _playercamera) (Variables|Default|GetUse%20Distance))) 5.0 "TraceTypeQuery1" true _outactors "None" true "(R=1.000000,G=0.683189,B=0.733152,A=1.000000)" "(R=0.652964,G=1.000000,B=0.636609,A=1.000000)"))
  (if _returnvalue_2
    (bind _asuse (Utilities|Casting|CastToUse (.HitActor (Collision|BreakHitResult _outhit)))
      (:then
        (Variables|Default|SetUsable%20Valid (Math|Boolean|ANDBoolean (Variables|/Game/Horror/Blueprints/Core/Use.Use_C|GetInteractionEnabled _asuse) (Utilities|IsValid (.HitComponent (Collision|BreakHitResult _outhit))) (Utilities|Enum|Equal(Enum) (Collision|GetCollisionObjectType (.HitComponent (Collision|BreakHitResult _outhit))) "ECC_GameTraceChannel1"))))
      (:CastFailed
        (Variables|Default|SetUsable%20Valid false :!label _label)))
    (else
      (goto _label))))