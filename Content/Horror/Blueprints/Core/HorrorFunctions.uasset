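; HorrorFunctions is a set of shared helper functions for a horror game's player and world queries.
; GetPlayer finds the HorrorEvents child actor on the player pawn, printing an attachment warning if the cast fails.
; PlayerInput uses it to enable or disable input on both pawn and HorrorEvents.
; A separate search loops over all actors of a class and returns the one nearest the player character, with a success flag.
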(fn GetPlayer
  (bind _filteredarray (Utilities|Array|FilterArray (Actor|GetAllChildActors (Game|Player|GetPlayerPawn 0) true) "/Game/Horror/Blueprints/Core/HorrorEvents.HorrorEvents_C"))
  (bind _ashorror_events (Utilities|Casting|CastToHorrorEvents (Utilities|Array|Get(acopy) _filteredarray))
    (:then
      _)
    (:CastFailed
      (Development|PrintString 0 "Attach HorrorEvents Blueprint to players Camera!")))
  (return _ashorror_events))

(fn PlayerInput
  (params (Enable :type Boolean))
  (bind _returnvalue (Game|Player|GetPlayerPawn 0))
  (bind _returnvalue_2 (Game|GetPlayerController 0))
  (bind _as_master (CallFunction|GetPlayer))
  (if Enable
    (Input|EnableInput _returnvalue _returnvalue_2)
    (else
      (Input|DisableInput _returnvalue _returnvalue_2))))

(fn NearestActortoPlayerOfClass
  (params (Actor%20Class :type Actor%20Class%20Reference))
  (bind _outactors (Actor|GetAllActorsOfClass 0 Actor%20Class))
  (LocalVariables|SetLocalFoundActor (> (Utilities|Array|Length _outactors) 0))
  (Utilities|IsValid (Utilities|Array|Get(acopy) _outactors)
    (:Is%20Valid
      (LocalVariables|SetLocalNearestActor (Utilities|Array|Get(acopy) _outactors))
      (LocalVariables|SetLocalFloatComparison (Transformation|GetDistanceTo (Utilities|Array|Get(acopy) _outactors) (Game|GetPlayerCharacter 0)))
      (for _array_element _outactors
        (Utilities|IsValid _array_element
          (:Is%20Valid
            (if (< (Transformation|GetDistanceTo _array_element (Game|GetPlayerCharacter 0)) (LocalVariables|GetLocalFloatComparison))
              (LocalVariables|SetLocalFloatComparison (Transformation|GetDistanceTo _array_element (Game|GetPlayerCharacter 0)))
              (LocalVariables|SetLocalNearestActor _array_element)))))
      (return (LocalVariables|GetLocalFoundActor) (LocalVariables|GetLocalNearestActor)))))